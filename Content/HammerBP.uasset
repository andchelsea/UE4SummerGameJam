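; HammerBP is a grabbable hammer that doubles as a pointer for choosing a weapon at an anvil.
; When its WidgetInteraction hovers an anvil weapon selection widget, it starts the owning Anvil's game with that widget's WeaponType, with no click needed.
; Pickup stops physics on the skeletal mesh and attaches it to the given component, while Drop re-enables physics and detaches the actor.
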(event OnHoveredWidgetChanged(WidgetInteraction)
  (params (WidgetComponent :type Widget%20Component%20Object%20Reference) (PreviousWidgetComponent :type Widget%20Component%20Object%20Reference))
  (bind _asanvil_weapon_selecton_widget_bp (Utilities|Casting|CastToAnvilWeaponSelectonWidgetBP (UserInterface|GetUserWidgetObject WidgetComponent)))
  (bind _asanvil (Utilities|Casting|CastToAnvil (Components|GetOwner WidgetComponent)))
  (Class|Anvil|StartGame _asanvil (Variables|/Game/FirstPersonCPP/Blueprints/UI/AnvilWeaponSelectonWidgetBP.AnvilWeaponSelectonWidgetBP_C|GetWeaponType _asanvil_weapon_selecton_widget_bp)))

(event EventBeginPlay)

(event Collision|EventActorBeginOverlap
  (params (OtherActor :type Actor%20Object%20Reference)))

(event EventTick
  (params (DeltaSeconds :type Float%20%28single-precision%29)))

(event EventPickup
  (params (AttachTo :type Scene%20Component%20Object%20Reference) (isLeft :type Boolean))
  (bind _skeletal_mesh (Variables|Default|GetSkeletal%20Mesh))
  (Physics|SetSimulatePhysics _skeletal_mesh false)
  (Transformation|AttachComponentToComponent _skeletal_mesh AttachTo "None" "KeepWorld" "KeepWorld" "KeepWorld" false))

(event EventDrop
  (Physics|SetSimulatePhysics (Variables|Default|GetSkeletal%20Mesh) true)
  (Transformation|DetachFromActor "KeepWorld" "KeepWorld" "KeepWorld"))

(fn ConstructionScript)